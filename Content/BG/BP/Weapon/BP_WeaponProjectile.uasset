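; BP_WeaponProjectile is a weapon projectile that pushes physics objects and damages monsters.
; On hit, it applies a velocity-scaled impulse to simulating-physics components, then destroys itself.
; On collision-component overlap, it applies fixed point damage only to actors whose class is exactly BP_Monster, crediting player pawn 0, and destroys itself whatever it touches.
; Both events print debug strings.
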(event `self.ReceiveHit`
  (params (MyComp :type "PrimitiveComponent Object Reference") (Other :type "Actor Object Reference") (OtherComp :type "PrimitiveComponent Object Reference") (bSelfMoved :type Boolean) (HitLocation :type "Vector Structure") (HitNormal :type "Vector Structure") (NormalImpulse :type "Vector Structure") (Hit :type "HitResult Structure (by ref)"))
  ;[1 1 1] 우리가 부딪힌 모든 물리 개체에 물리 충격을 추가합니다.
  (`KismetSystemLibrary.PrintString` "물리충격")
  (if (`SceneComponent.IsSimulatingPhysics` OtherComp "None")
    (`PrimitiveComponent.AddImpulseAtLocation` OtherComp (* (`self.GetVelocity`) 100.0) (`self.K2_GetActorLocation`) "None")
    (`self.K2_DestroyActor`) ; Then destroy this projectile
  ))

(event `self.CollisionComponent.OnComponentBeginOverlap`
  (params (OverlappedComponent :type "PrimitiveComponent Object Reference") (OtherActor :type "Actor Object Reference") (OtherComp :type "PrimitiveComponent Object Reference") (OtherBodyIndex :type Integer) (bFromSweep :type Boolean) (SweepResult :type "HitResult Structure (by ref)"))
  ;[1 1 1] 닿으면 AI가 데미지를 입는다.
  (`KismetSystemLibrary.PrintString` "오버랩!")
  (if (== (`GameplayStatics.GetObjectClass` OtherActor) "/Game/BG/BP/AI/BP_Monster.BP_Monster_C")
    (`KismetSystemLibrary.PrintString` "Hit")
    (`GameplayStatics.ApplyPointDamage` OtherActor 20.0 (`self.K2_GetActorLocation`) SweepResult null (`GameplayStatics.GetPlayerPawn` 0)))
  (`self.K2_DestroyActor`))

(fn `UserConstructionScript`)