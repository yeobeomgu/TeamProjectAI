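; BP_Light is a pickup item, apparently a handheld light adapted from weapon-firing logic, that attaches to BP_TestPlayer's spine_05 socket on sphere overlap.
; The pickup also binds an event to the player's OnUseItem dispatcher.
; OnLightProjectile calls LightServer, which spawns a BP_TestPlayer (not a projectile class) at the Ammo socket using camera rotation.
; LightServer also calls a sound multicast event, emits AI noise and plays a rifle-shoot montage.
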(event `self.SphereCollision.OnComponentBeginOverlap`
  (params (OverlappedComponent :type "PrimitiveComponent Object Reference") (OtherActor :type "Actor Object Reference") (OtherComp :type "PrimitiveComponent Object Reference") (OtherBodyIndex :type Integer) (bFromSweep :type Boolean) (SweepResult :type "HitResult Structure (by ref)"))
  ;[0 0.07435 1] 이걸 우리 캐릭터로 변경
  (bind _asbp_test_player (cast `/Game/BG/BP/BP_TestPlayer` OtherActor))
  (set `self.CharacterReference` _asbp_test_player)
  (`self.K2_AttachToComponent` self (`Character.Mesh` (`self.CharacterReference`)) "spine_05" "KeepRelative" "KeepRelative" "KeepRelative" true)
  (add `/Game/BG/BP/BP_TestPlayer.OnUseItem` (`self.CharacterReference`) (`|CreateDelegate` :!event `OnLightProjectile`)))

(event `OnLightProjectile`
  (`self.LightServer`))

(event `LightServer`
  (bind _returnvalue (`PlayerCameraManager.GetCameraRotation` (`GameplayStatics.GetPlayerCameraManager` 0)))
  (bind _returnvalue_2 (+ (`SceneComponent.GetSocketLocation` (`self.SkeletalMesh`) "Ammo") (`KismetMathLibrary.GreaterGreater_VectorRotator` (`self.ProjevtileOffest`) _returnvalue)))
  (`|SpawnActorFromClass` "/Game/BG/BP/BP_TestPlayer.BP_TestPlayer_C" (`KismetMathLibrary.MakeTransform` _returnvalue_2 _returnvalue) "Undefined" "OverrideRootScale" null null)
  (`self.Play Sound Multicaset` null _returnvalue_2)
  (`self.MakeNoise` 1.0 (`GameplayStatics.GetPlayerPawn` 0) (`self.K2_GetActorLocation`))
  ;[1 1 1] 라이트를 잡은 애니메이션동작
  (`AnimInstance.Montage_Play` (`SkeletalMeshComponent.GetAnimInstance` (`Character.Mesh` (`self.CharacterReference`))) "/Game/FirstPersonArms/Animations/FP_Rifle_Shoot_Montage.FP_Rifle_Shoot_Montage" 1.0 "MontageLength" 0.0 true))

(event `Play Sound Multicaset`
  (params (Sound :type "SoundBase Object Reference") (Location :type "Vector Structure"))
  (`GameplayStatics.PlaySoundAtLocation` Sound Location (struct) 1.0 1.0 0.0 null null null null))

(fn `UserConstructionScript`)